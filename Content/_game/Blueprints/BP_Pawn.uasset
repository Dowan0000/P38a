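; BP_Pawn is a player-controlled flying craft that constantly moves along its forward vector and fires rockets.
; Tick adds forward movement input and spins both wings around their local roll axis, scaled by delta time.
; Pitch and Roll axes rotate the body locally without delta-time scaling, while Accelerate raises FloatingPawnMovement's max speed while held.
; Shoot spawns a BP_Rocket at the Arrow component's world transform.
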(event `self.ReceiveTick`
  (params (DeltaSeconds :type "Float (single-precision)"))
  ;[1 1 1] Wing Rotation
  (`self.WingRotation` (`self.LeftWing`))
  (`self.WingRotation` (`self.RightWing`))
  ;[1 1 1] Move Forward
  (`self.AddMovementInput` (`self.GetActorForwardVector`)))

(event `InputAxis|Pitch`
  (params (AxisValue :type "Float (single-precision)"))
  ;[1 1 1] Pitch and Roll Rotate
  (`self.K2_AddActorLocalRotation` (`KismetMathLibrary.MakeRotator` 0.0 (* (`KismetMathLibrary.FClamp` AxisValue -1.0) (`self.BodyRotationRate`)))))

(event `InputAction|Accelerate`
  (params (Key :type "Key Structure"))
  ;[1 1 1] Accelerate
  (:`Pressed`
    (set `FloatingPawnMovement.MaxSpeed` 3000.0 (`self.FloatingPawnMovement`)))
  (:`Released`
    (set `FloatingPawnMovement.MaxSpeed` 500.0 (`self.FloatingPawnMovement`))))

(event `InputAxis|Roll`
  (params (AxisValue :type "Float (single-precision)"))
  ;[1 1 1] Pitch and Roll Rotate
  (`self.K2_AddActorLocalRotation` (`KismetMathLibrary.MakeRotator` (* (`KismetMathLibrary.FClamp` AxisValue -1.0) (`self.BodyRotationRate`)))))

(event `InputAction|Shoot`
  (params (Key :type "Key Structure"))
  ;[1 1 1] Spawn Rocket
  (:`Pressed`
    (`|SpawnActorFromClass` "/Game/_game/Blueprints/BP_Rocket.BP_Rocket_C" (`SceneComponent.K2_GetComponentToWorld` (`self.Arrow`)) "Undefined" "OverrideRootScale" null null)))

(fn `UserConstructionScript`)

(fn `WingRotation`
  (params (self2 :type "SceneComponent Object Reference"))
  (`SceneComponent.K2_AddLocalRotation` self2 (`KismetMathLibrary.MakeRotator` (* (`GameplayStatics.GetWorldDeltaSeconds`) (`self.WingRotationSpeed`))) false false))